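; Procedural mine layout generator that grows connected rooms from a first room on BeginPlay, then populates them with rats.
; It pre-measures room entrances with temporary spawns, then makes 40 attempts to align random allowed rooms to queued BP_Mine_Spawner doors, rejecting colliding spawns.
; Leftover doors get dead ends where a box trace is clear.
; Collected spawners provide rat spawn points and a goal location, currently only debug-drawn.
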(event EventBeginPlay
  (CallFunction|SetupPlacementsandMeasurements)
  (for _index (range 0 40)
    (CallFunction|PlaceNewRooms))
  (CallFunction|CleanUpRooms)
  (for _array_element (Variables|Default|GetSpawners)
    (if (Utilities|Enum|Equal(Enum) (Variables|/Game/Geometry/Generator/BP_Mine_Spawner.BP_Mine_Spawner_C|GetSpawnType _array_element) "NewEnumerator5")
      (if (> (Math|Vector|VectorLength (+ (Transformation|GetActorLocation) (Transformation|GetActorLocation _array_element))) (Variables|Default|GetGoalDistance))
        (Variables|Default|SetGoalDistance (Math|Vector|VectorLength (+ (Transformation|GetActorLocation) (Transformation|GetActorLocation _array_element))))
        (Variables|Default|SetGoalLoc (Transformation|GetActorLocation _array_element))
        (Variables|Default|SetGoalDoor _array_element))))
  (Rendering|Debug|DrawDebugSphere (Variables|Default|GetGoalLoc) 1e+02 12 "(R=1.000000,G=1.000000,B=1.000000,A=1.000000)" 1e+02 3.0)
  (Utilities|FlowControl|Delay 0.2)
  (for _array_element_2 (Variables|Default|GetSpawners)
    (if (or (Utilities|Enum|Equal(Enum) (Variables|/Game/Geometry/Generator/BP_Mine_Spawner.BP_Mine_Spawner_C|GetSpawnType _array_element_2) "NewEnumerator0") (Utilities|Enum|Equal(Enum) (Variables|/Game/Geometry/Generator/BP_Mine_Spawner.BP_Mine_Spawner_C|GetSpawnType _array_element_2) "NewEnumerator1"))
      (bind _returnvalue (Game|SpawnActorfromClass "/Game/AI/Enemies/AI_Character_Rat.AI_Character_Rat_C" (Math|Transform|MakeTransform (.location (Transformation|GetActorTransform _array_element_2)) (.rotation (Transformation|GetActorTransform _array_element_2)) "1,1,1") "Undefined" 0 10 0))
      (bind _asai_character_rat (Utilities|Casting|CastToAI_Character_Rat _returnvalue))
      (Variables|/Game/AI/Enemies/AI_Character_Base.AI_Character_Base_C|SetLevelSetByGenerator _asai_character_rat 10)
      (Default|InitParentSetup _asai_character_rat))))

(event Collision|EventActorBeginOverlap
  (params (OtherActor :type Actor%20Object%20Reference)))

(event EventTick
  (params (DeltaSeconds :type Float%20%28single-precision%29)))

(fn ConstructionScript)

(fn FindTransform
  (params (Key :type BP%20Room%20Parent%20Class%20Reference%20%28by%20ref%29))
  (bind _selected_door (Variables|Default|GetSelected%20Door))
  (bind _roomenterancetrans (Variables|Default|GetRoomEnteranceTrans))
  (bind _returnvalue (Transformation|GetActorTransform _selected_door))
  (bind _value (Utilities|Map|Find _roomenterancetrans Key))
  (bind _returnvalue_2 (- (.yaw (.rotation _returnvalue)) (.yaw (.rotation _value))))
  (return (+ (.location _returnvalue) (Math|Vector|RotateVectorAroundAxis (.location _value) _returnvalue_2 "0, 0,1.000000")) (+ _returnvalue_2 1.8e+02)))

(fn SelectNewRoomtoPlace
  (bind _allowedrooms (Variables|Default|GetAllowedRooms))
  (bind _roomsallowedtoplace (LocalVariables|GetRoomsAllowedToPlace))
  (bind _roomsallowedtoplace_2 (LocalVariables|GetRoomsAllowedToPlace))
  (bind _returnvalue (Utilities|Array|Length _roomsallowedtoplace))
  (bind _keys (Utilities|Map|Keys _allowedrooms))
  (for _array_element _keys
    (if (!= (.Value (Utilities|Map|Find _allowedrooms _array_element)) 0)
      (Utilities|Array|Add _roomsallowedtoplace_2 _array_element)))
  (if (> _returnvalue 0)
    (return (Utilities|Array|Get(acopy) _roomsallowedtoplace_2 (Math|Random|RandomIntegerinRange 0 (- _returnvalue 1))) true)
    (else
      (return 0 false))))

(fn RegisterNewDoors
  (params (RoomJustSpawned :type Actor%20Object%20Reference))
  (for _array_element (Actor|GetAllChildActors RoomJustSpawned true)
    (bind _asbp_mine_spawner (Utilities|Casting|CastToBP_Mine_Spawner _array_element))
    (if (and (Utilities|Enum|Equal(Enum) (Variables|/Game/Geometry/Generator/BP_Mine_Spawner.BP_Mine_Spawner_C|GetSpawnType _asbp_mine_spawner) "NewEnumerator8") (!= (Variables|/Game/Geometry/Generator/BP_Mine_Spawner.BP_Mine_Spawner_C|GetDoorID _asbp_mine_spawner) 0))
      (Utilities|Array|Add (Variables|Default|GetUnprocessedDoors) _asbp_mine_spawner)
      (elif (not (Utilities|Enum|Equal(Enum) (Variables|/Game/Geometry/Generator/BP_Mine_Spawner.BP_Mine_Spawner_C|GetSpawnType _asbp_mine_spawner) "NewEnumerator8"))
        (Utilities|Array|Add (Variables|Default|GetSpawners) _asbp_mine_spawner)))))

(fn ManageProcessedDoors
  (Utilities|Array|RemoveIndex (Variables|Default|GetUnprocessedDoors))
  (Variables|Default|SetSelected%20Door (Utilities|Array|Get(acopy) (Variables|Default|GetUnprocessedDoors))))

(fn TakeInitialMeasurements
  (bind _deadend (Variables|Default|GetDeadEnd))
  (bind _keys (Utilities|Map|Keys (Variables|Default|GetAllowedRooms)))
  (for _array_element _keys
    (bind _returnvalue (Game|SpawnActorfromClass _array_element (Math|Transform|MakeTransform "0, 0, 0" "0, 0, 0" "1,1,1") "AlwaysSpawn" 0 0))
    (bind _array_element_2 (Utilities|Array|ForEachLoopwithBreak (Actor|GetAllChildActors _returnvalue true) :!label _label)
      (:LoopBody
        (bind _asbp_mine_spawner (Utilities|Casting|CastToBP_Mine_Spawner _array_element_2))
        (if (and (Utilities|Enum|Equal(Enum) (Variables|/Game/Geometry/Generator/BP_Mine_Spawner.BP_Mine_Spawner_C|GetSpawnType _asbp_mine_spawner) "NewEnumerator8") (== (Variables|/Game/Geometry/Generator/BP_Mine_Spawner.BP_Mine_Spawner_C|GetDoorID _asbp_mine_spawner) 0))
          (Utilities|Map|Add (Variables|Default|GetRoomEnteranceTrans) _array_element (Transformation|GetActorTransform _asbp_mine_spawner))
          (goto _label Break)))
      (:Completed
        (Actor|DestroyActor _returnvalue))))
  (bind _returnvalue_2 (Game|SpawnActorfromClass _deadend (Math|Transform|MakeTransform "0, 0, 0" "0, 0, 0" "1,1,1") "AlwaysSpawn" 0 0))
  (bind _array_element_3 (Utilities|Array|ForEachLoopwithBreak (Actor|GetAllChildActors _returnvalue_2 true) :!label _label_2)
    (:LoopBody
      (bind _asbp_mine_spawner_2 (Utilities|Casting|CastToBP_Mine_Spawner _array_element_3))
      (if (and (Utilities|Enum|Equal(Enum) (Variables|/Game/Geometry/Generator/BP_Mine_Spawner.BP_Mine_Spawner_C|GetSpawnType _asbp_mine_spawner_2) "NewEnumerator8") (== (Variables|/Game/Geometry/Generator/BP_Mine_Spawner.BP_Mine_Spawner_C|GetDoorID _asbp_mine_spawner_2) 0))
        (Utilities|Map|Add (Variables|Default|GetRoomEnteranceTrans) _deadend (Transformation|GetActorTransform _asbp_mine_spawner_2))
        (goto _label_2 Break)))
    (:Completed
      (Variables|Default|SetDeadEndBounds (.BoxExtent (Collision|GetComponentBounds (Variables|/Game/Geometry/Generator/BP_Room_Parent.BP_Room_Parent_C|GetBox _returnvalue_2))))
      (Actor|DestroyActor _returnvalue_2))))

(fn PlaceFirstRoom
  (bind _returnvalue (Game|SpawnActorfromClass (Variables|Default|GetFirstRoom) (Math|Transform|MakeTransform (Transformation|GetActorLocation) "0, 0, 0" "1,1,1") "Undefined" 0 0))
  (for _array_element (Actor|GetAllChildActors _returnvalue true)
    (bind _asbp_mine_spawner (Utilities|Casting|CastToBP_Mine_Spawner _array_element))
    (if (Utilities|Enum|Equal(Enum) (Variables|/Game/Geometry/Generator/BP_Mine_Spawner.BP_Mine_Spawner_C|GetSpawnType _asbp_mine_spawner) "NewEnumerator8")
      (Utilities|Array|Add (Variables|Default|GetUnprocessedDoors) _asbp_mine_spawner)
      (else
        (Utilities|Array|Add (Variables|Default|GetSpawners) _asbp_mine_spawner)))))

(fn SetupPlacementsandMeasurements
  (bind _unprocesseddoors (Variables|Default|GetUnprocessedDoors))
  (bind _output (Utilities|Array|Get(acopy) _unprocesseddoors))
  (CallFunction|PlaceFirstRoom)
  (CallFunction|TakeInitialMeasurements)
  (Utilities|IsValid _output
    (:Is%20Valid
      (Variables|Default|SetSelected%20Door _output))))

(fn PlaceNewRooms
  (bind (_roomtoplace _successful_) (CallFunction|SelectNewRoomtoPlace))
  (if _successful_
    (bind _returnvalue (Game|SpawnActorfromClass _roomtoplace (Math|Transform|MakeTransform (.Loc (CallFunction|FindTransform _roomtoplace)) (Math|Rotator|MakeRotator 0.0 0.0 (.Yaw (CallFunction|FindTransform _roomtoplace))) "1,1,1") "DontSpawnIfColliding" 0 0))
    (Utilities|IsValid _returnvalue
      (:Is%20Valid
        (Utilities|Array|Add (Variables|Default|GetUnprocessedRooms) _returnvalue)
        (CallFunction|RegisterNewDoors _returnvalue)
        (CallFunction|ManageProcessedDoors)))))

(fn CleanUpRooms
  (for (_array_element _array_index) (Variables|Default|GetUnprocessedDoors)
    (Variables|Default|SetSelected%20Door _array_element)
    (CallFunction|HandleDeadEnds)
    (Actor|DestroyActor _array_element))
  (for _array_element_2 (Variables|Default|GetUnprocessedRooms)
    (Collision|SetCollisionResponsetoAllChannels (Variables|/Game/Geometry/Generator/BP_Room_Parent.BP_Room_Parent_C|GetBox _array_element_2) "ECR_Overlap")
    (Collision|SetCollisionEnabled (Variables|/Game/Geometry/Generator/BP_Room_Parent.BP_Room_Parent_C|GetRoomMesh _array_element_2) "QueryAndPhysics")))

(fn HandleDeadEnds
  (bind _deadendbounds (Variables|Default|GetDeadEndBounds))
  (bind _selected_door (Variables|Default|GetSelected%20Door))
  (bind _deadend (Variables|Default|GetDeadEnd))
  (bind _returnvalue (Transformation|GetActorLocation _selected_door))
  (bind _returnvalue_2 (Transformation|GetActorForwardVector _selected_door))
  (bind (_x _y _z) (Math|Vector|BreakVector _deadendbounds))
  (bind (_loc _yaw) (CallFunction|FindTransform _deadend))
  (bind _returnvalue_3 (* _returnvalue_2 _x))
  (bind _returnvalue_4 (+ _returnvalue _returnvalue_3 (Math|Vector|MakeVector 0.0 0.0 _z)))
  (bind _returnvalue_5 (Class|KismetSystemLibrary|BoxTraceSingleforObjects _returnvalue_4 _returnvalue_4 _deadendbounds (Math|Rotator|MakeRotator 0.0 0.0 (.yaw (Transformation|GetActorRotation _selected_door))) (Utilities|Array|MakeArray "ObjectTypeQuery1" "ObjectTypeQuery2") false 0 "Persistent" true))
  (if (not _returnvalue_5)
    (bind _returnvalue_6 (Game|SpawnActorfromClass _deadend (Math|Transform|MakeTransform _loc (Math|Rotator|MakeRotator 0.0 0.0 _yaw) "1,1,1") "Undefined" 0 0))
    (Utilities|Array|Add (Variables|Default|GetUnprocessedRooms) _returnvalue_6)
    (for _array_element (Actor|GetAllChildActors _returnvalue_6 false)
      (bind _asbp_mine_spawner (Utilities|Casting|CastToBP_Mine_Spawner _array_element))
      (if (Utilities|Enum|NotEqual(Enum) (Variables|/Game/Geometry/Generator/BP_Mine_Spawner.BP_Mine_Spawner_C|GetSpawnType _asbp_mine_spawner) "NewEnumerator8")
        (Utilities|Array|Add (Variables|Default|GetSpawners) _asbp_mine_spawner)))))