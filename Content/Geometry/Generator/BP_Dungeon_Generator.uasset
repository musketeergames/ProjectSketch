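; Procedural dungeon generator actor that spawns a start room at its location on BeginPlay, then attempts two random rooms from AllowedRooms.
; It briefly spawns each allowed room class to cache entrance offsets.
; Door-type BP_Mine_Spawner children supply the selected door (ID 0) and a door queue.
; New rooms derive position from the selected door and yaw from the queue head, which is consumed even when collision blocks spawning.
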(event EventBeginPlay
  (CallFunction|PlaceStartRoom)
  (for _index (range 0 1)
    (CallFunction|PlaceNewRoom)))

(event Collision|EventActorBeginOverlap
  (params (OtherActor :type Actor%20Object%20Reference)))

(event EventTick
  (params (DeltaSeconds :type Float%20%28single-precision%29)))

(fn ConstructionScript)

(fn PlaceStartRoom
  (bind _returnvalue (Game|SpawnActorfromClass (Variables|Default|GetStartRoom) (Math|Transform|MakeTransform (Transformation|GetActorLocation) "0, 0, 0" "1,1,1") "AlwaysSpawn" 0 0))
  (CallFunction|StoreActorMeasurements _returnvalue)
  (Variables|Default|SetSelectedRoom _returnvalue)
  (CallFunction|RegisterNewDoors _returnvalue true))

(fn RegisterNewSpawners
  (params (Room :type BP%20Room%20Parent%20Object%20Reference))
  (for _array_element (Actor|GetAllChildActors Room false)
    (bind _asbp_mine_spawner (Utilities|Casting|CastToBP_Mine_Spawner _array_element))
    (if (Utilities|Enum|NotEqual(Enum) (Variables|/Game/Geometry/Generator/BP_Mine_Spawner.BP_Mine_Spawner_C|GetSpawnType _asbp_mine_spawner) "NewEnumerator8")
      (Utilities|Array|Add (Variables|Default|GetSpawnerInfo) (Utilities|Struct|MakeSpawner_Info (Transformation|GetActorLocation _asbp_mine_spawner) (Transformation|GetActorRotation _asbp_mine_spawner) (Variables|/Game/Geometry/Generator/BP_Mine_Spawner.BP_Mine_Spawner_C|GetSpawnType _asbp_mine_spawner) (Variables|/Game/Geometry/Generator/BP_Mine_Spawner.BP_Mine_Spawner_C|GetFlavorDic _asbp_mine_spawner))))))

(fn RegisterNewDoors
  (params (Room :type BP%20Room%20Parent%20Object%20Reference) (StoreEnteranceDoor? :type Boolean))
  (for _array_element (Actor|GetAllChildActors Room false)
    (bind _asbp_mine_spawner (Utilities|Casting|CastToBP_Mine_Spawner _array_element))
    (if (Utilities|Enum|Equal(Enum) (Variables|/Game/Geometry/Generator/BP_Mine_Spawner.BP_Mine_Spawner_C|GetSpawnType _asbp_mine_spawner) "NewEnumerator8")
      (if (== (Variables|/Game/Geometry/Generator/BP_Mine_Spawner.BP_Mine_Spawner_C|GetDoorID _asbp_mine_spawner) 0)
        (Variables|Default|SetSelectedDoorTransform (Math|Transform|MakeTransform (Transformation|GetActorLocation _asbp_mine_spawner) (Transformation|GetActorRotation _asbp_mine_spawner)))
        (else
          (Utilities|Array|Add (Variables|Default|GetUnusedDoors) _asbp_mine_spawner)
          (Utilities|Array|Add (Variables|Default|GetDoorsInfo) (Utilities|Struct|MakeSpawner_Info (Transformation|GetActorLocation _asbp_mine_spawner) (Transformation|GetActorRotation _asbp_mine_spawner) (Variables|/Game/Geometry/Generator/BP_Mine_Spawner.BP_Mine_Spawner_C|GetSpawnType _asbp_mine_spawner) (Variables|/Game/Geometry/Generator/BP_Mine_Spawner.BP_Mine_Spawner_C|GetFlavorDic _asbp_mine_spawner) (Variables|/Game/Geometry/Generator/BP_Mine_Spawner.BP_Mine_Spawner_C|GetDoorID _asbp_mine_spawner))))))))

(fn SelectNewRoomtoPlace
  (bind _validroomsleft (LocalVariables|GetValidRoomsLeft))
  (bind _keys (Utilities|Map|Keys (Variables|Default|GetAllowedRooms)))
  (for _array_element _keys
    (Utilities|Array|Add (LocalVariables|GetValidRoomsLeft) _array_element))
  (if (not (> (Utilities|Array|Length (LocalVariables|GetValidRoomsLeft)) 0))
    (return false "/Game/Geometry/Generator/BP_Room_Parent.BP_Room_Parent_C")
    (else
      (return true (Utilities|Array|Get(acopy) _validroomsleft (Math|Random|RandomIntegerinRange 0 (- (Utilities|Array|Length _validroomsleft) 1)))))))

(fn PlaceNewRoom
  (bind (_successful_ _roomtoplace) (CallFunction|SelectNewRoomtoPlace))
  (if _successful_
    (bind _transform (CallFunction|FindTransform _roomtoplace))
    (bind _returnvalue (Game|SpawnActorfromClass _roomtoplace _transform "DontSpawnIfColliding" 0 0))
    (Utilities|Array|RemoveIndex (Variables|Default|GetUnusedDoors))
    (Utilities|Array|RemoveIndex (Variables|Default|GetDoorsInfo))
    (Utilities|IsValid _returnvalue
      (:Is%20Valid
        (CallFunction|RegisterNewDoors _returnvalue false)
        (Variables|Default|SetSelectedRoom _returnvalue)))))

(fn FindTransform
  (params (Class :type BP%20Room%20Parent%20Class%20Reference%20%28by%20ref%29))
  (bind _selecteddoortransform (Variables|Default|GetSelectedDoorTransform))
  (bind _enteranceoffset (Variables|Default|GetEnteranceOffset))
  (bind _value (Utilities|Map|Find _enteranceoffset Class))
  (Development|PrintString (Utilities|String|ToString(Vector) (.location _selecteddoortransform)))
  (return (Math|Transform|MakeTransform (+ (Math|Vector|RotateVectorAroundAxis (.location _value) (+ (.yaw (.rotation _value)) 1.8e+02) "0, 0,1.000000") (.location _selecteddoortransform)) (Math|Rotator|MakeRotator 0.0 0.0 (+ (- (.yaw (.WorldRot (Utilities|Struct|BreakSpawner_Info (Utilities|Array|Get(acopy) (Variables|Default|GetDoorsInfo))))) (.yaw (.rotation _value))) 1.8e+02)))))

(fn StoreActorMeasurements
  (params (FirstRoom :type BP%20Room%20Parent%20Object%20Reference))
  (bind (_class _measurementinfo _doorsinfo _enteranceoffsetreturn) (Default|TakeMeasurements FirstRoom))
  (Utilities|Map|Add (Variables|Default|GetEnteranceOffset) _class _enteranceoffsetreturn)
  (bind _keys (Utilities|Map|Keys (Variables|Default|GetAllowedRooms)))
  (for _array_element _keys
    (bind _returnvalue (Game|SpawnActorfromClass _array_element (Math|Transform|MakeTransform "0, 0, 0") "AlwaysSpawn" 0 0))
    (bind (_class_2 _measurementinfo_2 _doorsinfo_2 _enteranceoffsetreturn_2) (Default|TakeMeasurements _returnvalue))
    (Utilities|Map|Add (Variables|Default|GetEnteranceOffset) _class_2 _enteranceoffsetreturn_2)
    (Actor|DestroyActor _returnvalue)))

(fn SelectLastRoom)