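; BP_Room_Parent is a base room actor for procedural level generation, apparently for a mine, that positions itself at a door and can be replaced.
; SettleIntoPlace finds a specific type of BP_Mine_Spawner child, stores the door transform and ID, then rotates and shifts the room to align that spawner.
; ShouldIDie box-traces the room's bounds for world objects.
; RoomTooBigRepealAndReplace spawns a dead end at the stored transform and destroys the room.
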(event EventBeginPlay)

(event Collision|EventActorBeginOverlap
  (params (OtherActor :type Actor%20Object%20Reference)))

(event EventTick
  (params (DeltaSeconds :type Float%20%28single-precision%29)))

(fn ConstructionScript)

(fn SettleIntoPlace
  (bind _returnvalue (Transformation|GetActorRotation))
  (bind _returnvalue_2 (Transformation|GetActorLocation))
  (bind _array_element (Utilities|Array|ForEachLoopwithBreak (Actor|GetComponentsByClass "/Script/Engine.ChildActorComponent") :!label _label)
    (:LoopBody
      (bind _asbp_mine_spawner (Utilities|Casting|CastToBP_Mine_Spawner (Variables|/Script/Engine.ChildActorComponent|GetChildActor _array_element)))
      (if (Utilities|Enum|Equal(Enum) (Variables|/Game/Geometry/Generator/BP_Mine_Spawner.BP_Mine_Spawner_C|GetSpawnType _asbp_mine_spawner) "NewEnumerator8")
        (Utilities|FlowControl|Sequence
          (:then_0
            (goto _label Break))
          (:then_1
            (Variables|Default|SetDesiredDoorLoc _returnvalue_2)
            (Variables|Default|SetDesiredDoorRot (Math|Rotator|MakeRotator 0.0 0.0 (+ (.yaw _returnvalue) 1.8e+02)))
            (Transformation|SetActorRotation (Math|Rotator|MakeRotator 0.0 0.0 (+ (- (.yaw (Transformation|GetActorRotation _asbp_mine_spawner)) (.yaw _returnvalue)) 2.7e+02)))
            (Transformation|SetActorLocation (+ (Transformation|GetActorLocation) (- _returnvalue_2 (Transformation|GetActorLocation (Variables|/Script/Engine.ChildActorComponent|GetChildActor _array_element)))) false false)))))
    (:Completed
      (Variables|Default|SetEnteranceID (Variables|/Game/Geometry/Generator/BP_Mine_Spawner.BP_Mine_Spawner_C|GetDoorID _asbp_mine_spawner)))))

(fn ShouldIDie?
  (bind _box (Variables|Default|GetBox))
  (bind (_origin _boxextent) (Collision|GetComponentBounds _box))
  (bind _returnvalue (Class|KismetSystemLibrary|BoxTraceSingleforObjects _origin _origin _boxextent "0, 0, 0" (Utilities|Array|MakeArray "ObjectTypeQuery1" "ObjectTypeQuery2") false 0 "Persistent" true))
  (return _returnvalue (Variables|Default|GetEnteranceID)))

(fn RoomTooBigRepealandReplace
  (params (DeadEnd :type BP%20Room%20Parent%20Class%20Reference))
  (bind _desireddoorloc (Variables|Default|GetDesiredDoorLoc))
  (bind _returnvalue (Game|SpawnActorfromClass DeadEnd (Math|Transform|MakeTransform _desireddoorloc (Variables|Default|GetDesiredDoorRot)) "AlwaysSpawn" 0 0))
  (Rendering|Debug|DrawDebugSphere _desireddoorloc 1e+02 12 "(R=0.000000,G=0.103376,B=1.000000,A=1.000000)" 1e+02 3.0)
  (Utilities|IsValid _returnvalue
    (:Is%20Valid
      (Actor|DestroyActor))
    (:Is%20Not%20Valid
      (Development|PrintString "Help"))))