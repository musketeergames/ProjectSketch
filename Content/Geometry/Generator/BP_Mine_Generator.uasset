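; Procedural mine generator actor that builds a layout of connected room meshes on BeginPlay.
; It briefly spawns each room class to cache measurements, then places the start room.
; A fixed loop picks random rooms with remaining quota, aligns them at a Selector moved through queued doors, box-traces for overlap and adds per-class HISM instances.
; An older actor-spawning path remains but is disconnected, and debug drawing is left on.
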(event EventBeginPlay
  (CallFunction|StoreActorMeasurements)
  (Spawning|PlaceStartRoom)
  (for _index (range 0 50)
    (CallFunction|PlaceNewRoom)
    (CallFunction|SelectNextDoor)))

(fn ConstructionScript)

(fn PlaceStartRoom
  (bind _returnvalue (Transformation|GetActorRotation))
  (bind _storedmeasurements (Variables|Default|GetStoredMeasurements))
  (bind _startroom (Variables|Default|GetStartRoom))
  (bind _value (Utilities|Map|Find _storedmeasurements _startroom))
  (bind (_spawnerinfo _mesh) (Utilities|Struct|BreakMeasurements_Info _value))
  (bind _array_element (Utilities|Array|ForEachLoopwithBreak _spawnerinfo :!label _label)
    (:LoopBody
      (if (Utilities|Enum|Equal(Enum) (.Type (Utilities|Struct|BreakSpawner_Info _array_element)) "NewEnumerator8")
        (Utilities|FlowControl|Sequence
          (:then_0
            (goto _label Break))
          (:then_1
            (bind _returnvalue_2 (AddComponent|AddStaticMeshComponent false (Math|Transform|MakeTransform (.WorldLoc (Utilities|Struct|BreakSpawner_Info _array_element)) (Math|Rotator|MakeRotator (.roll _returnvalue) (.pitch _returnvalue) (+ (- (.yaw _returnvalue) (.Yaw (Math|Rotator|BreakRotator (.WorldRot (Utilities|Struct|BreakSpawner_Info _array_element))))) 9e+01)))))
            (Components|StaticMesh|SetStaticMesh _returnvalue_2 _mesh)
            (Transformation|SetRelativeTransform (Variables|Default|GetSelector) (Math|Transform|MakeTransform "0, 0, 0" (Math|Rotator|MakeRotator 0.0 0.0 (- (.yaw _returnvalue) (.Yaw (Math|Rotator|BreakRotator (.WorldRot (Utilities|Struct|BreakSpawner_Info _array_element))))))) false true)))))))

(fn AddtoArray
  (params (Actor :type BP%20Room%20Parent%20Object%20Reference))
  (bind _roommesh (Variables|/Game/Geometry/Generator/BP_Room_Parent.BP_Room_Parent_C|GetRoomMesh Actor))
  (bind _meshcount (Variables|Default|GetMeshCount))
  (bind (_value _returnvalue) (Utilities|Map|Find _meshcount _roommesh))
  (if _returnvalue
    (Utilities|Map|Add _meshcount 0 (+ _value 1))
    (else
      (Utilities|Map|Add _meshcount _roommesh 1))))

(fn StoreSpawnData
  (bind _outactors (Actor|GetAllActorsOfClass "/Game/Geometry/Generator/BP_Room_Parent.BP_Room_Parent_C"))
  (for _array_element _outactors
    (for _array_element_2 (Actor|GetComponentsByClass _array_element "/Script/Engine.ChildActorComponent")
      (bind _asbp_mine_spawner (Utilities|Casting|CastToBP_Mine_Spawner (Variables|/Script/Engine.ChildActorComponent|GetChildActor _array_element_2)))
      (if (Utilities|Enum|NotEqual(Enum) (Variables|/Game/Geometry/Generator/BP_Mine_Spawner.BP_Mine_Spawner_C|GetSpawnType _asbp_mine_spawner) "NewEnumerator8")
        (Utilities|Array|Add (Variables|Default|GetSpawnerData) (Utilities|Struct|MakeSpawner_Info (Transformation|GetActorLocation _asbp_mine_spawner) (Transformation|GetActorRotation _asbp_mine_spawner) (Variables|/Game/Geometry/Generator/BP_Mine_Spawner.BP_Mine_Spawner_C|GetSpawnType _asbp_mine_spawner) (Variables|/Game/Geometry/Generator/BP_Mine_Spawner.BP_Mine_Spawner_C|GetFlavorDic _asbp_mine_spawner)))))))

(fn SelectNewRoomtoPlace
  (bind _allowedrooms (Variables|Default|GetAllowedRooms))
  (bind _validroomsleft (LocalVariables|GetValidRoomsLeft))
  (bind _keys (Utilities|Map|Keys _allowedrooms))
  (for _array_element _keys
    (if (!= (.Value (Utilities|Map|Find _allowedrooms _array_element)) 0)
      (Utilities|Array|Add (LocalVariables|GetValidRoomsLeft) _array_element)))
  (if (not (> (Utilities|Array|Length (LocalVariables|GetValidRoomsLeft)) 0))
    (return false "/Game/Geometry/Generator/BP_Room_Parent.BP_Room_Parent_C")
    (else
      (return true (Utilities|Array|Get(acopy) _validroomsleft (Math|Random|RandomIntegerinRange 0 (- (Utilities|Array|Length _validroomsleft) 1)))))))

(fn FindTransform
  (params (RoomToPlace :type BP%20Room%20Parent%20Class%20Reference))
  (bind _storedmeasurements (Variables|Default|GetStoredMeasurements))
  (bind _selector (Variables|Default|GetSelector))
  (bind _value (Utilities|Map|Find _storedmeasurements RoomToPlace))
  (bind _returnvalue (Transformation|GetWorldTransform _selector))
  (bind (_spawnerinfo _mesh _materials _bounds _meshorigindisplacement) (Utilities|Struct|BreakMeasurements_Info _value))
  (bind _return (CallFunction|CalculateMeshOffsetPerRotation _meshorigindisplacement (.yaw (.rotation _returnvalue))))
  (bind (_x _y) (Math|Vector|BreakVector _meshorigindisplacement))
  (bind (_x_2 _y_2 _z) (Math|Vector|BreakVector _return))
  (for _array_element _spawnerinfo
    (if (Utilities|Enum|Equal(Enum) (.Type (Utilities|Struct|BreakSpawner_Info _array_element)) "NewEnumerator8")
      (if (== (.DoorID (Utilities|Struct|BreakSpawner_Info _array_element)) 0)
        (LocalVariables|SetEnteranceTrans (Math|Transform|MakeTransform (.WorldLoc (Utilities|Struct|BreakSpawner_Info _array_element)) (.WorldRot (Utilities|Struct|BreakSpawner_Info _array_element))))
        (else
          (Utilities|Array|Add (Variables|Default|GetUnusedDoorLocalTransforms) (Math|Transform|MakeTransform (.WorldLoc (Utilities|Struct|BreakSpawner_Info _array_element)) (.WorldRot (Utilities|Struct|BreakSpawner_Info _array_element))))))))
  (CallFunction|ConvertLocalDoorstoWorld (Math|Transform|MakeTransform (+ (.location _returnvalue) (.location (LocalVariables|GetEnteranceTrans)) "0, 0, 0") (Math|Rotator|MakeRotator 0.0 0.0 (+ (+ (- (.yaw (.rotation _returnvalue)) (.yaw (.rotation (LocalVariables|GetEnteranceTrans)))) 1.8e+02) (.yaw (Transformation|GetActorRotation))))))
  (Development|PrintString (Utilities|String|ToString(Float) (.yaw (.rotation _returnvalue))))
  (return (Math|Transform|MakeTransform (+ (Math|Vector|MakeVector _x_2 _y_2 _z) (.location _returnvalue) (.location (LocalVariables|GetEnteranceTrans))) (Math|Rotator|MakeRotator 0.0 0.0 (+ (+ (- (.yaw (.rotation _returnvalue)) (.yaw (.rotation (LocalVariables|GetEnteranceTrans)))) 1.8e+02) (.yaw (Transformation|GetActorRotation))))) (Math|Transform|MakeTransform (Math|Vector|MakeVector (+ (.X (Math|Vector|BreakVector (+ (Math|Vector|MakeVector _x_2 _y_2 _z) (.location _returnvalue) (.location (LocalVariables|GetEnteranceTrans))))) _x) (+ (.Y (Math|Vector|BreakVector (+ (Math|Vector|MakeVector _x_2 _y_2 _z) (.location _returnvalue) (.location (LocalVariables|GetEnteranceTrans))))) _y) (+ (.Z (Math|Vector|BreakVector (+ (Math|Vector|MakeVector _x_2 _y_2 _z) (.location _returnvalue) (.location (LocalVariables|GetEnteranceTrans))))) (.Z (Math|Vector|BreakVector _bounds)))))))

(fn RegisterNewDoors
  (params (Actor :type BP%20Room%20Parent%20Object%20Reference) (ExcludeID :type Integer))
  (DataManagement|AddtoArray Actor)
  (for _array_element (Actor|GetComponentsByClass Actor "/Script/Engine.ChildActorComponent")
    (bind _asbp_mine_spawner (Utilities|Casting|CastToBP_Mine_Spawner (Variables|/Script/Engine.ChildActorComponent|GetChildActor _array_element)))
    (if (and (Utilities|Enum|Equal(Enum) (Variables|/Game/Geometry/Generator/BP_Mine_Spawner.BP_Mine_Spawner_C|GetSpawnType _asbp_mine_spawner) "NewEnumerator8") (!= (Variables|/Game/Geometry/Generator/BP_Mine_Spawner.BP_Mine_Spawner_C|GetDoorID _asbp_mine_spawner) ExcludeID))
      (Utilities|Array|Add (Variables|Default|GetDoorsData) (Utilities|Struct|MakeSpawner_Info (Transformation|GetActorLocation _asbp_mine_spawner) (Transformation|GetActorRotation _asbp_mine_spawner) "NewEnumerator8" (Variables|/Game/Geometry/Generator/BP_Mine_Spawner.BP_Mine_Spawner_C|GetFlavorDic _asbp_mine_spawner)))
      (Utilities|Array|Add (Variables|Default|GetUnusedDoors) _asbp_mine_spawner))))

(fn SendNextRoomtoDoors
  (bind _unuseddoors (Variables|Default|GetUnusedDoors))
  (bind _allowedrooms (Variables|Default|GetAllowedRooms))
  (bind (_successful_ _roomtoplace) (Selecting|SelectNewRoomtoPlace))
  (if _successful_
    (for (_array_element _array_index) _unuseddoors
      (bind _roomjustspawned (Default|SpawnRoom _array_element _roomtoplace))
      (bind _output_get (Variables|Default|SetRoomJustSpawned _roomjustspawned))
      (Utilities|Array|RemoveIndex _unuseddoors _array_index)
      (bind (_return _enteranceused) (Default|ShouldIDie? _output_get))
      (if _return
        (Default|RoomTooBigRepealandReplace _output_get (Variables|Default|GetDeadEndRoom))
        (else
          (Utilities|Map|Add _allowedrooms _roomtoplace (- (.Value (Utilities|Map|Find _allowedrooms _roomtoplace)) 1))
          (Math|Integer|IncrementInt (Variables|Default|GetIntRoomsPlaced)
            (:%20%20
              (DataManagement|RegisterNewDoors _output_get _enteranceused))))))
    (else
      (Variables|Default|SetMaxRoomsAllowed 0))))

(fn InitMeshComps
  (params (Key :type BP%20Room%20Parent%20Class%20Reference%20%28by%20ref%29))
  (bind _returnvalue (Math|Transform|MakeTransform "0, 0, 0"))
  (bind _allowedrooms (Variables|Default|GetAllowedRooms))
  (bind _storedmeasurements (Variables|Default|GetStoredMeasurements))
  (bind (_value _returnvalue_2) (Utilities|Map|Find _allowedrooms Key))
  (bind _value_2 (Utilities|Map|Find _storedmeasurements Key))
  (bind _mesh (Utilities|Struct|BreakMeasurements_Info _value_2))
  (if _returnvalue_2
    (if (> _value 1)
      (bind _returnvalue_3 (AddComponent|AddHierarchicalInstancedStaticMeshComponent false _returnvalue))
      (Components|StaticMesh|SetStaticMesh _returnvalue_3 _mesh)
      (else
        (bind _returnvalue_4 (AddComponent|AddStaticMeshComponent false _returnvalue :!label _label))
        (Components|StaticMesh|SetStaticMesh _returnvalue_4 _mesh)))
    (else
      (goto _label))))

(fn StoreActorMeasurements
  (bind _returnvalue (Math|Transform|MakeTransform "0, 0, 0"))
  (bind _returnvalue_2 (Game|SpawnActorfromClass (Variables|Default|GetStartRoom) _returnvalue "AlwaysSpawn" 0 0))
  (bind (_class _measurementinfo) (Default|TakeMeasurements _returnvalue_2))
  (Utilities|Map|Add (Variables|Default|GetStoredMeasurements) _class _measurementinfo)
  (Actor|DestroyActor _returnvalue_2)
  (bind _keys (Utilities|Map|Keys (Variables|Default|GetAllowedRooms)))
  (for _array_element _keys
    (bind _returnvalue_3 (Game|SpawnActorfromClass _array_element _returnvalue "AlwaysSpawn" 0 0))
    (bind (_class_2 _measurementinfo_2) (Default|TakeMeasurements _returnvalue_3))
    (Utilities|Map|Add (Variables|Default|GetStoredMeasurements) _class_2 _measurementinfo_2)
    (Actor|DestroyActor _returnvalue_3)))

(fn PlaceNewRoom
  (bind (_successful_ _roomtoplace) (Selecting|SelectNewRoomtoPlace))
  (if _successful_
    (bind (_returnvalue _origintransform) (CallFunction|FindTransform _roomtoplace))
    (CallFunction|AddRoomInstance _returnvalue _roomtoplace _origintransform)))

(fn AddRoomInstance
  (params (RoomTransform :type Transform) (Class :type BP%20Room%20Parent%20Class%20Reference) (OriginTransform :type Transform))
  (bind _allowedrooms (Variables|Default|GetAllowedRooms))
  (bind _meshinstancesdic (Variables|Default|GetMeshInstancesDic))
  (bind (_value _returnvalue) (Utilities|Map|Find _meshinstancesdic Class))
  (bind _oktospawn (CallFunction|ShouldThisRoomSpawn? OriginTransform Class))
  (if _oktospawn
    (Utilities|Map|Add _allowedrooms Class (- (.Value (Utilities|Map|Find _allowedrooms Class)) 1))
    (if _returnvalue
      (Class|InstancedStaticMeshComponent|AddInstanceWorldSpace _value RoomTransform)
      (else
        (bind _returnvalue_2 (AddComponent|AddHierarchicalInstancedStaticMeshComponent false (Math|Transform|MakeTransform "0, 0, 0")))
        (Components|StaticMesh|SetStaticMesh _returnvalue_2 (.Mesh (Utilities|Struct|BreakMeasurements_Info (.Value (Utilities|Map|Find (Variables|Default|GetStoredMeasurements) Class)))))
        (Class|InstancedStaticMeshComponent|AddInstanceWorldSpace _returnvalue_2 RoomTransform)
        (Utilities|Map|Add (Variables|Default|GetMeshInstancesDic) Class _returnvalue_2)))))

(fn ShouldThisRoomSpawn?
  (params (Trans :type Transform) (Room :type BP%20Room%20Parent%20Class%20Reference))
  (bind _returnvalue (Class|KismetSystemLibrary|BoxTraceSingleforObjects (.location Trans) (.location Trans) (.Bounds (Utilities|Struct|BreakMeasurements_Info (.Value (Utilities|Map|Find (Variables|Default|GetStoredMeasurements) Room)))) (.rotation Trans) (Utilities|Array|MakeArray "ObjectTypeQuery1" "ObjectTypeQuery2") false 0 "Persistent" true)) ; Might need to fix
  (return (not _returnvalue)))

(fn SelectNextDoor
  (bind _unuseddoorworldtransforms (Variables|Default|GetUnusedDoorWorldTransforms))
  (bind _output (Utilities|Array|Get(acopy) _unuseddoorworldtransforms))
  (Transformation|SetWorldLocationAndRotation (Variables|Default|GetSelector) (.location _output) (.rotation _output) false false)
  (Rendering|Debug|DrawDebugSphere (.location _output) 1e+02 12 "(R=1.000000,G=1.000000,B=1.000000,A=1.000000)" 1e+02 3.0)
  (Utilities|Array|RemoveIndex _unuseddoorworldtransforms))

(fn ConvertLocalDoorstoWorld
  (params (RoomTransform :type Transform))
  (for _array_element (Variables|Default|GetUnusedDoorLocalTransforms)
    (Utilities|Array|Add (Variables|Default|GetUnusedDoorWorldTransforms) (Math|Transform|MakeTransform (- (.location RoomTransform) (.Location (Math|Transform|BreakTransform _array_element))) (Math|Rotator|MakeRotator 0.0 0.0 (+ (.yaw (.rotation RoomTransform)) (.yaw (.Rotation (Math|Transform|BreakTransform _array_element))))))))
  (Utilities|Array|Clear (Variables|Default|GetUnusedDoorLocalTransforms)))

(fn CalculateMeshOffsetPerRotation
  (params (Offset :type Vector) (Yaw :type Float%20%28single-precision%29))
  (bind (_x _y) (Math|Vector|BreakVector Offset))
  (bind (_x_2 _y_2) (Math|Vector|BreakVector Offset))
  (return (Utilities|Select :Index (Math|Float|Round (/ Yaw 9e+01)) :Option%200 (Math|Vector|MakeVector (* _y_2 -1.0) _x_2 0.0) :Option%201 (* Offset -1.0) :Option%202 (Math|Vector|MakeVector _y (* _x -1.0) 0.0) :Option%203 Offset)))