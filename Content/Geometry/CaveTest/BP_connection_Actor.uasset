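; Connection point actor for cave room layouts that caps itself with a BP_Room_Dead_End.
; When active, PlaceDeadEnd checks the first connection actor overlapping Sphere3 to set Connected, then casts it to BP_Room_Dead_End.
; A dead end with a valid connection deactivates this point, while a failed cast does nothing.
; Otherwise it spawns a yaw-rotated dead end here, passing Connected as ConnectionValid and setting Placed.
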(event EventBeginPlay)

(event Collision|EventActorBeginOverlap
  (params (OtherActor :type Actor%20Object%20Reference)))

(event EventTick
  (params (DeltaSeconds :type Float%20%28single-precision%29)))

(fn ConstructionScript)

(fn PlaceDeadEnd
  (bind _returnvalue (Transformation|GetActorTransform))
  (bind _sphere3 (Variables|Default|GetSphere3))
  (bind _overlappingactors (Collision|GetOverlappingActors _sphere3 "BP_connection_Actor_C" :!class /Script/Engine.PrimitiveComponent))
  (bind (_location _rotation _scale) (Math|Transform|BreakTransform _returnvalue))
  (bind _item (Utilities|Array|Get(acopy) _overlappingactors))
  (if (Variables|Default|GetActive)
    (if (Utilities|IsValid _item)
      (Variables|Default|SetConnected true)
      (bind _asbp_room_dead_end (Utilities|Casting|CastToBP_Room_Dead_End _item))
      (if (Variables|/Game/Geometry/CaveTest/BP_Room_Dead_End.BP_Room_Dead_End_C|GetConnectionValid _asbp_room_dead_end)
        (Variables|Default|SetActive false)
        (else
          (bind _returnvalue_2 (Game|SpawnActorfromClass "/Game/Geometry/CaveTest/BP_Room_Dead_End.BP_Room_Dead_End_C" (Math|Transform|MakeTransform _location (Math|Rotator|MakeRotator 0.0 0.0 (+ (.yaw _rotation) 2.7e+02)) _scale) "Undefined" 0 0 :!label _label))
          (Variables|Default|SetPlaced true)
          (Variables|/Game/Geometry/CaveTest/BP_Room_Dead_End.BP_Room_Dead_End_C|SetConnectionValid _returnvalue_2 (Variables|Default|GetConnected))))
      (else
        (Variables|Default|SetConnected false)
        (goto _label)))))