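; Procedural cave slide actor that builds a randomly winding, descending tube in its construction script.
; BuildSpline appends downward points that go straight or turn 90 degrees left or right, using the previous tangent to track facing; the last segment always runs straight.
; CreateMesh lays collidable tube spline meshes between points.
; AddLights spaces point lights evenly along the spline's length.
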(event EventBeginPlay)

(event Collision|EventActorBeginOverlap
  (params (OtherActor :type Actor%20Object%20Reference)))

(event EventTick
  (params (DeltaSeconds :type Float%20%28single-precision%29)))

(fn ConstructionScript
  (CallFunction|BuildSpline)
  (CallFunction|CreateMesh)
  (CallFunction|AddLights))

(fn BuildSpline
  (bind _returnvalue (Math|Vector|MakeVector 7e+02 0.0 -3.5e+02))
  (bind _returnvalue_2 (Math|Vector|MakeVector 7e+02 0.0 -3.5e+02))
  (bind _spline (Variables|Default|GetSpline))
  (for _index (range 1 (Variables|Default|GetSegments))
    (if (== _index 1)
      (Spline|SetLocationatSplinePoint _spline 1 _returnvalue_2 "Local" true)
      (Variables|Default|SetPreviousSplinePoint _returnvalue_2)
      (Spline|SetTangentatSplinePoint _spline 0 _returnvalue "Local" true)
      (Variables|Default|SetPreviousSplineTangent _returnvalue)
      (elif (== _index (Variables|Default|GetSegments))
        (CallFunction|AddPointForward _index :!label _label)
        (elif (Math|Random|RandomBoolwithWeight 0.5)
          (goto _label)
          (elif (Math|Random|RandomBool)
            (CallFunction|AddPointRight _index)
            (else
              (CallFunction|AddPointLeft _index))))))))

(fn CreateMesh
  (bind _spline (Variables|Default|GetSpline))
  (for _index (range 0 (- (Variables|Default|GetSegments) 1))
    (bind _returnvalue (AddComponent|AddSplineMeshComponent false (Math|Transform|MakeTransform "0, 0, 0")))
    (Components|StaticMesh|SetStaticMesh _returnvalue "/Game/Geometry/CaveTest/Slides/Tube.Tube")
    (Collision|SetCollisionEnabled _returnvalue "QueryAndPhysics")
    (SplineMesh|SetForwardAxis _returnvalue "Z" true)
    (SplineMesh|SetStartandEnd _returnvalue (.Location (Spline|GetLocationandTangentatSplinePoint _spline _index "Local")) (.Tangent (Spline|GetLocationandTangentatSplinePoint _spline _index "Local")) (.Location (Spline|GetLocationandTangentatSplinePoint _spline (+ _index 1) "Local")) (.Tangent (Spline|GetLocationandTangentatSplinePoint _spline (+ _index 1) "Local")) true :!class /Script/Engine.SplineMeshComponent)))

(fn AddPointForward
  (params (PointIndex :type Integer))
  (bind _direction (CallFunction|FindFacingDirection))
  (switch Utilities|FlowControl|Switch|SwitchonEDirections _direction
    (:NewEnumerator0
      (Spline|AddSplinePoint (Variables|Default|GetSpline) (+ (Variables|Default|GetPreviousSplinePoint) "700.000000,0.000000,-350.000000") "Local" true)
      (Variables|Default|SetPreviousSplinePoint (+ (Variables|Default|GetPreviousSplinePoint) "700.000000,0.000000,-350.000000"))
      (Spline|SetTangentatSplinePoint (Variables|Default|GetSpline) PointIndex (Variables|Default|GetPreviousSplineTangent) "Local" true))
    (:NewEnumerator1
      (Spline|AddSplinePoint (Variables|Default|GetSpline) (+ (Variables|Default|GetPreviousSplinePoint) "0.000000,700.000000,-350.000000") "Local" true)
      (Variables|Default|SetPreviousSplinePoint (+ (Variables|Default|GetPreviousSplinePoint) "0.000000,700.000000,-350.000000"))
      (Spline|SetTangentatSplinePoint (Variables|Default|GetSpline) PointIndex (Variables|Default|GetPreviousSplineTangent) "Local" true))
    (:NewEnumerator2
      (Spline|AddSplinePoint (Variables|Default|GetSpline) (+ (Variables|Default|GetPreviousSplinePoint) "-700.000000,0.000000,-350.000000") "Local" true)
      (Variables|Default|SetPreviousSplinePoint (+ (Variables|Default|GetPreviousSplinePoint) "-700.000000,0.000000,-350.000000"))
      (Spline|SetTangentatSplinePoint (Variables|Default|GetSpline) PointIndex (Variables|Default|GetPreviousSplineTangent) "Local" true))
    (:NewEnumerator3
      (Spline|AddSplinePoint (Variables|Default|GetSpline) (+ (Variables|Default|GetPreviousSplinePoint) "0.000000,-700.000000,-350.000000") "Local" true)
      (Variables|Default|SetPreviousSplinePoint (+ (Variables|Default|GetPreviousSplinePoint) "0.000000,-700.000000,-350.000000"))
      (Spline|SetTangentatSplinePoint (Variables|Default|GetSpline) PointIndex (Variables|Default|GetPreviousSplineTangent) "Local" true))))

(fn AddLights
  (bind _spline (Variables|Default|GetSpline))
  (for _index (range 0 (.ReturnValue (Math|Float|Division(WholeandRemainder) (Spline|GetSplineLength _spline) 8e+02)))
    (AddComponent|AddPointLightComponent false (Math|Transform|MakeTransform (Spline|GetLocationatDistanceAlongSpline _spline (* _index 8e+02) "Local")))))

(fn AddPointRight
  (params (PointIndex :type Integer))
  (bind _returnvalue (Math|Vector|MakeVector 7e+02 0.0 0.0))
  (bind _returnvalue_2 (Math|Vector|MakeVector 0.0 7e+02 0.0))
  (bind _returnvalue_3 (Math|Vector|MakeVector -7e+02 0.0 0.0))
  (bind _returnvalue_4 (Math|Vector|MakeVector 0.0 -7e+02 0.0))
  (bind _direction (CallFunction|FindFacingDirection))
  (switch Utilities|FlowControl|Switch|SwitchonEDirections _direction
    (:NewEnumerator0
      (Spline|AddSplinePoint (Variables|Default|GetSpline) (+ (Variables|Default|GetPreviousSplinePoint) "700.000000,350.000000,-350.000000") "Local" true)
      (Variables|Default|SetPreviousSplinePoint (+ (Variables|Default|GetPreviousSplinePoint) "700.000000,350.000000,-350.000000"))
      (Spline|SetTangentatSplinePoint (Variables|Default|GetSpline) PointIndex _returnvalue_2 "Local" true)
      (Variables|Default|SetPreviousSplineTangent _returnvalue_2))
    (:NewEnumerator1
      (Spline|AddSplinePoint (Variables|Default|GetSpline) (+ (Variables|Default|GetPreviousSplinePoint) "-350.000000,700.000000,-350.000000") "Local" true)
      (Variables|Default|SetPreviousSplinePoint (+ (Variables|Default|GetPreviousSplinePoint) "-350.000000,700.000000,-350.000000"))
      (Spline|SetTangentatSplinePoint (Variables|Default|GetSpline) PointIndex _returnvalue_3 "Local" true)
      (Variables|Default|SetPreviousSplineTangent _returnvalue_3))
    (:NewEnumerator2
      (Spline|AddSplinePoint (Variables|Default|GetSpline) (+ (Variables|Default|GetPreviousSplinePoint) "-700.000000,-350.000000,-350.000000") "Local" true)
      (Variables|Default|SetPreviousSplinePoint (+ (Variables|Default|GetPreviousSplinePoint) "-700.000000,-350.000000,-350.000000"))
      (Spline|SetTangentatSplinePoint (Variables|Default|GetSpline) PointIndex _returnvalue_4 "Local" true)
      (Variables|Default|SetPreviousSplineTangent _returnvalue_4))
    (:NewEnumerator3
      (Spline|AddSplinePoint (Variables|Default|GetSpline) (+ (Variables|Default|GetPreviousSplinePoint) "350.000000,-700.000000,-350.000000") "Local" true)
      (Variables|Default|SetPreviousSplinePoint (+ (Variables|Default|GetPreviousSplinePoint) "350.000000,-700.000000,-350.000000"))
      (Spline|SetTangentatSplinePoint (Variables|Default|GetSpline) PointIndex _returnvalue "Local" true)
      (Variables|Default|SetPreviousSplineTangent _returnvalue))))

(fn FindFacingDirection
  (bind _previoussplinetangent (Variables|Default|GetPreviousSplineTangent))
  (if (> (.x _previoussplinetangent) 0.0)
    (return "NewEnumerator0")
    (elif (< (.x _previoussplinetangent) 0.0)
      (return "NewEnumerator2")
      (elif (> (.y _previoussplinetangent) 0.0)
        (return "NewEnumerator1")
        (else
          (return "NewEnumerator3"))))))

(fn AddPointLeft
  (params (PointIndex :type Integer))
  (bind _returnvalue (Math|Vector|MakeVector -7e+02 0.0 0.0))
  (bind _returnvalue_2 (Math|Vector|MakeVector 0.0 -7e+02 0.0))
  (bind _returnvalue_3 (Math|Vector|MakeVector 7e+02 0.0 0.0))
  (bind _returnvalue_4 (Math|Vector|MakeVector 0.0 7e+02 0.0))
  (bind _direction (CallFunction|FindFacingDirection))
  (switch Utilities|FlowControl|Switch|SwitchonEDirections _direction
    (:NewEnumerator0
      (Spline|AddSplinePoint (Variables|Default|GetSpline) (+ (Variables|Default|GetPreviousSplinePoint) "700.000000,-350.000000,-350.000000") "Local" true)
      (Variables|Default|SetPreviousSplinePoint (+ (Variables|Default|GetPreviousSplinePoint) "700.000000,-350.000000,-350.000000"))
      (Spline|SetTangentatSplinePoint (Variables|Default|GetSpline) PointIndex _returnvalue_2 "Local" true)
      (Variables|Default|SetPreviousSplineTangent _returnvalue_2))
    (:NewEnumerator1
      (Spline|AddSplinePoint (Variables|Default|GetSpline) (+ (Variables|Default|GetPreviousSplinePoint) "350.000000,700.000000,-350.000000") "Local" true)
      (Variables|Default|SetPreviousSplinePoint (+ (Variables|Default|GetPreviousSplinePoint) "350.000000,700.000000,-350.000000"))
      (Spline|SetTangentatSplinePoint (Variables|Default|GetSpline) PointIndex _returnvalue_3 "Local" true)
      (Variables|Default|SetPreviousSplineTangent _returnvalue_3))
    (:NewEnumerator2
      (Spline|AddSplinePoint (Variables|Default|GetSpline) (+ (Variables|Default|GetPreviousSplinePoint) "-700.000000,350.000000,-350.000000") "Local" true)
      (Variables|Default|SetPreviousSplinePoint (+ (Variables|Default|GetPreviousSplinePoint) "-700.000000,350.000000,-350.000000"))
      (Spline|SetTangentatSplinePoint (Variables|Default|GetSpline) PointIndex _returnvalue_4 "Local" true)
      (Variables|Default|SetPreviousSplineTangent _returnvalue_4))
    (:NewEnumerator3
      (Spline|AddSplinePoint (Variables|Default|GetSpline) (+ (Variables|Default|GetPreviousSplinePoint) "-350.000000,-700.000000,-350.000000") "Local" true)
      (Variables|Default|SetPreviousSplinePoint (+ (Variables|Default|GetPreviousSplinePoint) "-350.000000,-700.000000,-350.000000"))
      (Spline|SetTangentatSplinePoint (Variables|Default|GetSpline) PointIndex _returnvalue "Local" true)
      (Variables|Default|SetPreviousSplineTangent _returnvalue))))