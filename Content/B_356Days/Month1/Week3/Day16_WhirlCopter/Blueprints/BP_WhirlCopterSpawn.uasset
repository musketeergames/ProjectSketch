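; BP_WhirlCopterSpawn is an actor that plays a repeating whirl copter sequence with a skeletal mesh animation and six whirl effects.
; On BeginPlay it starts the WhirlCopterTL timeline, whose event tracks activate the Whirl components, play the copter animation once, and later deactivate the effects and stop the animation.
; When the timeline finishes it restarts itself from the start, so the sequence cycles indefinitely.
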(event EventBeginPlay
  (Timeline|WhirlCopterTL Play
    (:Finished
      (Timeline|WhirlCopterTL PlayFromStart))
    (:Activate
      (Components|Activation|Activate (Variables|Default|GetWhirl1) false))
    (:Animation
      (Components|Animation|PlayAnimation (Variables|Default|GetWhirlCopter) "/Game/B_356Days/Month1/Week3/Day16_WhirlCopter/SkeletalMeshes/SKM_WhirlCopter_01_Anim.SKM_WhirlCopter_01_Anim" false))
    (:Deactivate
      (Components|Activation|Deactivate (Variables|Default|GetWhirl1))
      (Audio|Components|Audio|Stop (Variables|Default|GetWhirlCopter)))))

(fn ConstructionScript)